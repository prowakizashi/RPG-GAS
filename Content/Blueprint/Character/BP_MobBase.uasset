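; BP_MobBase is a mob character base Blueprint that handles spawn and dissolve visuals and attack-agnostic facing.
; On BeginPlay a timeline scales the mesh uniformly.
; Separate body and weapon timelines drive the "Dissolve" scalar on dynamic material instances passed into their start events.
; UpdateFacingTarget feeds a location to Motion Warping as the "FacingTarget" warp target.
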(event `self.ReceiveBeginPlay`
  (bind (_direction _scaletrack) (`Timeline|SpawnTimeline`)
    (:`Update`
      (`SceneComponent.SetRelativeScale3D` (`self.Mesh`) (`KismetMathLibrary.MakeVector` _scaletrack _scaletrack _scaletrack)))))

(event `self.StartDissolveTimeline`
  (params (DynamicMaterialInstance :type "MaterialInstanceDynamic Object Reference"))
  (bind (_direction _dissolvevalue) (`Timeline|DissolveTimeline`)
    (:`Update`
      (`MaterialInstanceDynamic.SetScalarParameterValue` DynamicMaterialInstance "Dissolve" _dissolvevalue))))

(event `self.StartWeaponDissolveTimeline`
  (params (DynamicMaterialInstance :type "MaterialInstanceDynamic Object Reference"))
  (bind (_direction _weapondissolvevalue) (`Timeline|DissolveWeaponTimeline`)
    (:`Update`
      (`MaterialInstanceDynamic.SetScalarParameterValue` DynamicMaterialInstance "Dissolve" _weapondissolvevalue))))

(fn `UpdateFacingTarget`
  (params (TargetLocation :type "Vector Structure (by ref)"))
  (`MotionWarpingComponent.AddOrUpdateWarpTargetFromLocation` (`self.MotionWarping`) "FacingTarget" TargetLocation)
  (return))

(fn `UserConstructionScript`)