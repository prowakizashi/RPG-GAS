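; BP_FlamePillar is a flame pillar actor that flickers its FireLight for an animated fire effect.
; On BeginPlay it randomly picks one of two intensity timelines and starts it after a random short delay, so multiple pillars vary in pattern and phase.
; The chosen timeline replays endlessly, and each update passes its value to ScaleFlameIntensity, which multiplies it by BaseIntensity to set the light's intensity.
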(event `self.ReceiveBeginPlay`
  (bind _returnvalue (`KismetMathLibrary.RandomFloatInRange` 0.0 2.0))
  (if (`KismetMathLibrary.RandomBool`)
    (`KismetSystemLibrary.Delay` _returnvalue)
    (bind (_direction _intensity) (`Timeline|FlameIntensity_1` :!label _label)
      (:`Update`
        (`self.ScaleFlameIntensity` _intensity))
      (:`Finished`
        (goto _label :!via `PlayFromStart`)))
    (else
      (`KismetSystemLibrary.Delay` _returnvalue)
      (bind (_direction_2 _intensity_2) (`Timeline|FlameIntensity_2` :!label _label_2)
        (:`Update`
          (`self.ScaleFlameIntensity` _intensity_2))
        (:`Finished`
          (goto _label_2 :!via `PlayFromStart`))))))

(fn `ScaleFlameIntensity`
  (params (Intensity :type "Float (double-precision)"))
  (`LightComponent.SetIntensity` (`self.FireLight`) (* Intensity (`self.BaseIntensity`))))

(fn `UserConstructionScript`)