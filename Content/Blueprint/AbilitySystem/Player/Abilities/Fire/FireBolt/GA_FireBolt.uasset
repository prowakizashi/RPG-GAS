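; Player Fire Bolt gameplay ability that casts a projectile toward the location under the mouse cursor.
; After committing, it reads the cursor hit from a target data task and tells the avatar to face that point.
; It then plays the cast montage while waiting for its Fire Bolt gameplay event, which spawns the projectile from the weapon socket.
; The ability ends when the montage completes, blends out, is interrupted or is cancelled.
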(event `self.K2_ActivateAbility`
  (bind _returnvalue (`self.K2_CommitAbility`))
  (if _returnvalue
    (bind (_asynctaskproxy _datahandle) (`TargetDataUnderMouseTask.CreateTargetDataUnderMouseTask`)
      (:`OnGetTargetData`
        (set `self.TargetLocation` (`.Location` (`GameplayStatics.BreakHitResult` (`AbilitySystemBlueprintLibrary.GetHitResultFromTargetData` _datahandle))))
        (message `CombatInterface.UpdateFacingTarget` (`self.GetAvatarActorFromActorInfo`) (`self.TargetLocation`))
        (`AbilityTask_WaitGameplayEvent.WaitGameplayEvent` (struct :`TagName` "Event.Montage.FireBolt") null true
          (:`then`
            (`AbilityTask_PlayMontageAndWait.CreatePlayMontageAndWaitProxy` "None" "/Game/DruidAssets/Characters/Aura/Animations/Abilities/AM_CastFireBolt.AM_CastFireBolt" 1.0 "None" false
              (:`OnCompleted`
                _)
              (:`OnBlendOut`
                _)
              (:`OnInterrupted`
                _)
              (:`OnCancelled`
                _))
            (`self.K2_EndAbility`))
          (:`EventReceived`
            (`self.SpawnProjectile` (`self.TargetLocation`) (`BlueprintGameplayTagLibrary.MakeLiteralGameplayTag` (struct :`TagName` "CombatSocket.Weapon")))))))))