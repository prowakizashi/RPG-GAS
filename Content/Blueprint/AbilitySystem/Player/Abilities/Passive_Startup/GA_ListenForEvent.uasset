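; Passive startup player ability that listens for gameplay events under the Attributes tag hierarchy and turns them into gameplay effects on its owner.
; Each received event creates a spec from EventBasedEffectClass.
; Every tag in EventsTags becomes a SetByCaller magnitude: the exact match gets the event's magnitude, all others zero.
; The spec is then applied to self, letting one effect class serve all listed events.
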(event `self.K2_ActivateAbility`
  (bind _returnvalue (`self.GetAbilitySystemComponentFromActorInfo`))
  (bind (_asynctaskproxy _payload) (`AbilityTask_WaitGameplayEvent.WaitGameplayEvent` (struct :`TagName` "Attributes") null false false)
    (:`EventReceived`
      (set `self.EffectSpec` (`AbilitySystemComponent.MakeOutgoingSpec` _returnvalue (`self.EventBasedEffectClass`) 0.0 (`AbilitySystemComponent.MakeEffectContext` _returnvalue)))
      (for _array_element (`self.EventsTags`)
        (bind (_eventtag _instigator _target _optionalobject _optionalobject2 _contexthandle _instigatortags _targettags _eventmagnitude) (break `GameplayEventData` _payload))
        (`AbilitySystemBlueprintLibrary.AssignTagSetByCallerMagnitude` (`self.EffectSpec`) _array_element (`KismetMathLibrary.SelectFloat` _eventmagnitude 0.0 (`BlueprintGameplayTagLibrary.MatchesTag` _array_element _eventtag true))))
      (`AbilitySystemComponent.BP_ApplyGameplayEffectSpecToSelf` (`self.GetAbilitySystemComponentFromActorInfo`) (`self.EffectSpec`)))))