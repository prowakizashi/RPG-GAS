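; Player Electrocute ability: a channeled lightning beam toward the mouse hit that chains to additional targets when the first is a combat actor.
; A montage event spawns ShockLoop gameplay cues, locks movement and starts a looping timer that pays cost and applies set-by-caller lightning damage.
; Cues sit on each struck target, or on the player without a valid one.
; Input release, failed cost or target death clears timer and cues and restores movement.
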(event `self.K2_ActivateAbility`
  (if (`KismetSystemLibrary.DoesImplementInterface` (`self.GetAvatarActorFromActorInfo`) "/Script/RPG.CombatInterface")
    ; Store Initial Data
    (bind (_asynctaskproxy _datahandle) (`TargetDataUnderMouseTask.CreateTargetDataUnderMouseTask`)
      (:`then`
        (`self.StoreMouseDataInfo` (`AbilitySystemBlueprintLibrary.GetHitResultFromTargetData` _datahandle))
        (`self.StoreOwnerVariables`)
        (`|ExecutionSequence`
          (:`then_0`
            (set `PlayerController.bShowMouseCursor` false (`self.OwnerPlayerController`))
            (message `CombatInterface.UpdateFacingTarget` (`self.GetAvatarActorFromActorInfo`) (`self.MouseHitLocation`))
            (`self.K2_ExecuteGameplayCue` (struct :`TagName` "GameplayCue.ShockBurst"))
            (`AbilityTask_PlayMontageAndWait.CreatePlayMontageAndWaitProxy` "None" (`self.Montage_Electrocute`)
              (:`then`
                (`AbilityTask_WaitGameplayEvent.WaitGameplayEvent` (struct :`TagName` "Event.Montage.Electrocute") null true
                  (:`EventReceived`
                    (`self.SpawnElectricBeam`)
                    (message `CombatInterface.SetInShockLoop` (`self.GetAvatarActorFromActorInfo`) true)
                    (`CharacterMovementComponent.DisableMovement` (`Character.CharacterMovement` (`self.OwnerCharacter`)))
                    (bind _returnvalue (`KismetSystemLibrary.K2_SetTimerDelegate` (delegate `DamageAndCost`) (`self.DamageDeltaTime`) true))
                    (set `self.DamageAndCostTimer` _returnvalue))))))
          (:`then_1`
            (`AbilityTask_WaitInputRelease.WaitInputRelease` false
              (:`OnRelease`
                (`self.PrepareToEndAbility`)
                (`self.K2_EndAbility`)))))))
    (else
      (`self.K2_EndAbility`))))

(event `DamageAndCost`
  (bind _returnvalue (`self.K2_CommitAbilityCost` false))
  (if _returnvalue
    (if (`self.TargetDead`)
      (`self.PrepareToEndAbility`)
      (`self.K2_EndAbility`)
      (else
        (`self.ApplyDamage`)))
    (else
      (`self.PrepareToEndAbility`)
      (`self.K2_EndAbility`))))

(fn `AddShockAdditionnalTarget`
  (params (AdditionnalTarget :type "Actor Object Reference"))
  (bind _additionnaltarget (`local.AdditionnalTarget`))
  (bind _returnvalue (`AbilitySystemBlueprintLibrary.MakeGameplayCueParameters` 0.0 0.0 (struct) (struct) (struct) (struct) (struct) (`Actor.K2_GetActorLocation` _additionnaltarget) (0.0 0.0 0.0) null null _additionnaltarget null 1 1 (`Actor.RootComponent` (`self.MouseHitActor`))))
  (`BlueprintMapLibrary.Map_Add` (`self.AdditionnalActorsToCueParams`) AdditionnalTarget _returnvalue)
  (`GameplayCueFunctionLibrary.AddGameplayCueOnActor` (`local.AdditionnalTarget`) (struct :`TagName` "GameplayCue.ShockLoop") _returnvalue))

(fn `ApplyDamage`
  (`self.ApplyDamageSingleTarget` (`self.MouseHitActor`))
  (for _array_element (`self.AdditionalTargets`)
    (`self.ApplyDamageSingleTarget` _array_element)))

(fn `ApplyDamageSingleTarget`
  (params (Actor :type "Actor Object Reference"))
  (bind _returnvalue (`self.GetAbilitySystemComponentFromActorInfo`))
  (bind _returnvalue_2 (`AbilitySystemBlueprintLibrary.GetAbilitySystemComponent` Actor))
  (bind _returnvalue_3 (`AbilitySystemBlueprintLibrary.AssignTagSetByCallerMagnitude` (`AbilitySystemComponent.MakeOutgoingSpec` _returnvalue (`self.DamageEffectClass`) (`KismetMathLibrary.Conv_IntToDouble` (`self.GetAbilityLevel`)) (`AbilitySystemComponent.MakeEffectContext` _returnvalue)) (struct :`TagName` "Damage.Lightning") (`self.GetDamageAtLevel`)))
  (`/Engine/EditorBlueprintResources/StandardMacros.IsValid` _returnvalue_2
    (:`Is Valid`
      (`AbilitySystemComponent.BP_ApplyGameplayEffectSpecToSelf` _returnvalue_2 _returnvalue_3))))

(fn `PrepareToEndAbility`
  (`KismetSystemLibrary.K2_ClearAndInvalidateTimerHandle` (`self.DamageAndCostTimer`))
  (set `PlayerController.bShowMouseCursor` true (`self.OwnerPlayerController`))
  (message `CombatInterface.SetInShockLoop` (`self.GetAvatarActorFromActorInfo`) false)
  (`CharacterMovementComponent.SetMovementMode` (`Character.CharacterMovement` (`self.OwnerCharacter`)) "MOVE_Walking" 0)
  (if (`self.FirstTargetImplementsInterface`)
    (`GameplayCueFunctionLibrary.RemoveGameplayCueOnActor` (`self.MouseHitActor`) (struct :`TagName` "GameplayCue.ShockLoop") (`self.FirstTargetCueParams`))
    (for _array_element (`self.AdditionalTargets`)
      (bind (_value _returnvalue) (`BlueprintMapLibrary.Map_Find` (`self.AdditionnalActorsToCueParams`) _array_element))
      (if _returnvalue
        (`GameplayCueFunctionLibrary.RemoveGameplayCueOnActor` _array_element (struct :`TagName` "GameplayCue.ShockLoop") _value)))
    (else
      (`GameplayCueFunctionLibrary.RemoveGameplayCueOnActor` (`self.GetAvatarActorFromActorInfo`) (struct :`TagName` "GameplayCue.ShockLoop") (`self.FirstTargetCueParams`)))))

(fn `SpawnElectricBeam`
  (locals (CueTarget :type "Actor Object Reference"))
  (`self.TraceFirstTarget` (`self.MouseHitLocation`))
  (bind _returnvalue (message `CombatInterface.GetWeapon` (`self.GetAvatarActorFromActorInfo`)))
  (set `self.FirstTargetCueParams` (`AbilitySystemBlueprintLibrary.MakeGameplayCueParameters` 0.0 0.0 (struct) (struct) (struct) (struct) (struct) (`self.MouseHitLocation`) (0.0 0.0 0.0) null null (`self.MouseHitActor`) null 1 1 _returnvalue))
  ; Is Mouse Hit Actor an Enemy ?
  (bind _output_get (set `self.FirstTargetImplementsInterface` (`KismetSystemLibrary.DoesImplementInterface` (`self.MouseHitActor`) "/Script/RPG.CombatInterface")))
  (if _output_get
    (set `local.CueTarget` (`self.MouseHitActor`)) ; Then the cue is carried by the Enemy
    (else
      (set `local.CueTarget` (`self.GetAvatarActorFromActorInfo`)) ; Then the cue is carried by the Player
    ))
  (`GameplayCueFunctionLibrary.AddGameplayCueOnActor` (`local.CueTarget`) (struct :`TagName` "GameplayCue.ShockLoop") (`self.FirstTargetCueParams`))
  (if (`self.FirstTargetImplementsInterface`)
    (bind _outadditionaltargets (`self.StoreAdditionnalTargets`))
    (bind _output_get_2 (set `self.AdditionalTargets` _outadditionaltargets))
    (for _array_element _output_get_2
      (`self.AddShockAdditionnalTarget` _array_element))))