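; GA_RangeAttack is a mob gameplay ability that performs a ranged attack on the avatar's current combat target.
; On activation it captures the target's location, turns the avatar to face it and plays a random tagged attack montage from the avatar.
; A gameplay event matching the montage tag spawns a projectile from the montage's socket toward that stored location.
; The ability ends when the montage completes, is interrupted or is cancelled, or immediately if no montage exists.
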(event `self.K2_ActivateAbility`
  (bind _returnvalue (`self.GetAvatarActorFromActorInfo`))
  (bind (_randomtaggedmontage_montage _randomtaggedmontage_impactsound _randomtaggedmontage_montagetag _randomtaggedmontage_sockettag) (break `TaggedMontage` (`self.RandomTaggedMontage`)))
  (bind _returnvalue_2 (message `MobInterface.GetCombatTarget` _returnvalue))
  (bind _output_get (set `self.TargetLocation` (`Actor.K2_GetActorLocation` _returnvalue_2)))
  (message `CombatInterface.UpdateFacingTarget` _returnvalue _output_get)
  (bind _returnvalue_3 (message `CombatInterface.GetAttackMontages` _returnvalue))
  (bind (_outitem _outindex) (`KismetArrayLibrary.Array_Random` _returnvalue_3))
  (if (>= _outindex 0)
    (bind _output_get_2 (set `self.RandomTaggedMontage` _outitem))
    (`AbilityTask_PlayMontageAndWait.CreatePlayMontageAndWaitProxy` "None" (break `TaggedMontage` _output_get_2) 1.0 "None" false
      (:`then`
        (`AbilityTask_WaitGameplayEvent.WaitGameplayEvent` _randomtaggedmontage_montagetag null true
          (:`EventReceived`
            (message `CombatInterface.GetAttackSocketLocation` (`self.GetAvatarActorFromActorInfo`) _randomtaggedmontage_sockettag)
            (`self.SpawnProjectile` (`self.TargetLocation`) _randomtaggedmontage_sockettag))))
      (:`OnCompleted`
        (`self.K2_EndAbility` :!label _label))
      (:`OnInterrupted`
        (goto _label))
      (:`OnCancelled`
        (goto _label)))
    (else
      (`self.K2_EndAbility`))))