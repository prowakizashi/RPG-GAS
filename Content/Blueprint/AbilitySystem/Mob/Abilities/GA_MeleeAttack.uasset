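; Gameplay Ability for mob melee attacks, instanced per actor, that damages living, non-friendly players.
; It turns the avatar toward its combat target and plays a random tagged montage, both through interface messages on the avatar.
; The montage's gameplay event triggers a small sphere query at the attack socket, damages valid targets and fires an impact cue on a hit.
; The ability then ends without stopping the montage.
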(event `self.K2_ActivateAbility`
  (bind _returnvalue (`self.GetAvatarActorFromActorInfo`))
  (bind _returnvalue_2 (`self.GetAvatarActorFromActorInfo`))
  (bind ((`MontageTag` _montagetag) (`SocketTag` _sockettag)) (break `TaggedMontage` (`self.RandomTaggedMontage`)))
  (set `self.bHasHitTarget` false) ; We have 1 instance per actor,\nso we reset variables on each activation
  (bind _returnvalue_3 (message `MobInterface.GetCombatTarget` _returnvalue_2))
  (message `CombatInterface.UpdateFacingTarget` _returnvalue_2 (`Actor.K2_GetActorLocation` _returnvalue_3))
  (bind _returnvalue_4 (message `CombatInterface.GetAttackMontages` _returnvalue_2))
  (bind (_outitem _outindex) (`KismetArrayLibrary.Array_Random` _returnvalue_4))
  (if (>= _outindex 0)
    (bind _output_get (set `self.RandomTaggedMontage` _outitem))
    (`AbilityTask_PlayMontageAndWait.CreatePlayMontageAndWaitProxy` "None" (break `TaggedMontage` _output_get) 1.0 "None" false
      (:`then`
        (`AbilityTask_WaitGameplayEvent.WaitGameplayEvent` _montagetag null true
          (:`EventReceived`
            (bind _returnvalue_5 (message `CombatInterface.GetAttackSocketLocation` _returnvalue _sockettag))
            (bind _output_get_2 (set `self.CombatSocketLocation` _returnvalue_5))
            (bind _outoverlappingplayers (`RPGAbilitySystemLibrary.GetAlivePlayersWithinRadius` (`|MakeArray` _returnvalue) 45.0 _output_get_2))
            (for _array_element _outoverlappingplayers
              (if (`RPGAbilitySystemLibrary.AreNotFriends` (`self.GetAvatarActorFromActorInfo`) _array_element)
                (`self.CauseDamage` _array_element)
                (set `self.bHasHitTarget` true)))
            (`|ExecutionSequence`
              (:`then_0`
                (if (`self.bHasHitTarget`)
                  (bind _returnvalue_6 (message `MobInterface.GetCombatTarget` (`self.GetAvatarActorFromActorInfo`)))
                  (`self.K2_ExecuteGameplayCueWithParams` (struct :`TagName` "GameplayCue.Melee.impact") (`AbilitySystemBlueprintLibrary.MakeGameplayCueParameters` 0.0 0.0 (struct) (struct) (struct) (`BlueprintGameplayTagLibrary.MakeGameplayTagContainerFromTag` (`.MontageTag` (break `TaggedMontage` (`self.RandomTaggedMontage`)))) (struct) (`self.CombatSocketLocation`) (0.0 0.0 0.0) null (`self.GetAvatarActorFromActorInfo`) _returnvalue_6))))
              (:`then_1`
                (`self.K2_EndAbility`))))))
      (:`OnCompleted`
        (`self.K2_EndAbility` :!label _label))
      (:`OnInterrupted`
        (goto _label))
      (:`OnCancelled`
        (goto _label)))
    (else
      (`self.K2_EndAbility`))))